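; Player controller for the in-game text chat, linking the player to the chat widget.
; On BeginPlay it waits via a zero-second Delay, then caches the chat widget from BP_ChatHUD.
; The T key toggles the mouse cursor and switches between game-and-UI and game-only input.
; SendMessage relays user and text to every BP_ChatController found, each passing it to its widget through AddMessage.
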(event Custom|ToggleChat
  ;[1 1 1] ToggleChat/Pressed T chat open
  (bind _output_get (Variables|Default|SetbShowMouseCursor (not (Variables|Default|GetbShowMouseCursor))))
  (if _output_get
    (Input|SetInputModeGameandUI self 0 "DoNotLock" true false)
    (else
      (Input|SetInputModeGameOnly self false))))

(event Custom|SendMessage
  (params (User :type Name) (Message :type Text))
  ;[1 1 1] Send Message
  (bind _outactors (Actor|GetAllActorsOfClass "BP_ChatController_C"))
  (for _array_element _outactors
    (Utilities|IsValid _array_element
      (:Is%20Valid
        (CallFunction|AddMessage _array_element User Message)))))

(event Custom|AddMessage
  (params (User :type Name) (Message :type Text))
  (Default|AddMessage (Variables|Default|GetChat_Widget) User Message))

(event EventBeginPlay
  ;[1 1 1] Chat HUD
  (Utilities|FlowControl|Delay 0.0)
  (bind _asbp_chat_hud (Utilities|Casting|CastToBP_ChatHUD (HUD|GetHUD)))
  (bind _output_get (Variables|Default|Set%20BP%20Chat%20HUD _asbp_chat_hud))
  (Variables|Default|SetChat_Widget (Variables|/Game/Blueprint/WidgetBP/BP_ChatHUD.BP_ChatHUD_C|GetChat_Widget _output_get)))

(event EventTick
  (params (DeltaSeconds :type Float%20%28single-precision%29)))

(event Input|KeyboardEvents|T
  (params (Key :type Key%20Structure :default "None"))
  ;[1 1 1] ToggleChat/Pressed T chat open
  (:Pressed
    (CallFunction|ToggleChat)))

(fn ConstructionScript)