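; Player character Blueprint that manages the ammo and HP HUD plus reload and knife cooldowns.
; BeginPlay creates the bullet count, bullet gauge and HP widgets, and update events map counts of 0 to 3 onto text and radial sliders.
; Reloading shows a temporary widget with a Timeline-driven material alpha, then re-enables firing and refills three bullets.
; Knife events use delays to re-enable firing and rotate the knife component back to a set pose.
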(event EventBeginPlay
  (bind _returnvalue (UserInterface|CreateWidget "/Game/KHJContents/UI/WB_BulCountNum.WB_BulCountNum_C"))
  (bind _output_get (Variables|Default|SetBulCountNumRef _returnvalue))
  (UserInterface|Viewport|AddtoViewport _output_get 0)
  (bind _returnvalue_2 (UserInterface|CreateWidget "/Game/KHJContents/UI/WB_BulCountUIR.WB_BulCountUIR_C"))
  (bind _output_get_2 (Variables|Default|SetBulCountRef _returnvalue_2))
  (UserInterface|Viewport|AddtoViewport _output_get_2 0)
  (bind _returnvalue_3 (UserInterface|CreateWidget "/Game/KHJContents/UI/WB_HPUIR.WB_HPUIR_C"))
  (bind _output_get_3 (Variables|Default|SetHPUIRefR _returnvalue_3))
  (UserInterface|Viewport|AddtoViewport _output_get_3 0))

(event Collision|EventActorBeginOverlap
  (params (OtherActor :type Actor%20Object%20Reference)))

(event EventTick
  (params (DeltaSeconds :type Float%20%28single-precision%29)))

(event EventResetFireCoolDown
  (bind _bulcountref (Variables|Default|GetBulCountRef))
  (bind _radialslider_93 (Variables|/Game/KHJContents/UI/WB_BulCountUIR.WB_BulCountUIR_C|GetRadialSlider_93 _bulcountref))
  (bind _returnvalue (UserInterface|CreateWidget "/Game/KHJContents/UI/WB_ReloadingUI.WB_ReloadingUI_C"))
  (Variables|Default|SetBulWidgetRef _returnvalue)
  (UserInterface|Viewport|AddtoViewport (Variables|Default|GetBulWidgetRef) 0)
  (bind _returnvalue_2 (Appearance|GetDynamicMaterial (Variables|/Game/KHJContents/UI/WB_ReloadingUI.WB_ReloadingUI_C|GetImage_0 (Variables|Default|GetBulWidgetRef)) :!class /Script/UMG.Image))
  (bind _uitrack (Timeline|Timeline PlayFromStart)
    (:Update
      (Rendering|Material|SetScalarParameterValue _returnvalue_2 "Alpha" _uitrack :!class /Script/Engine.MaterialInstanceDynamic))
    (:Finished
      (Widget|RemovefromParent (Variables|Default|GetBulWidgetRef))
      (Variables|Default|SetbCanFire true)
      (Variables|Default|SetcurBulletCount 3)
      (Variables|/Script/UMG.TextBlock|SetText (Variables|/Game/KHJContents/UI/WB_BulCountNum.WB_BulCountNum_C|Getcurbultext (Variables|Default|GetBulCountNumRef)) (Utilities|Text|ToText(Integer) (Variables|Default|GetcurBulletCount)))
      (Utilities|FlowControl|Sequence
        (:then_0
          (if (== (Variables|Default|GetcurBulletCount) 3)
            (Variables|/Script/AdvancedWidgets.RadialSlider|SetValue _radialslider_93 1.0)))
        (:then_1
          (if (== (Variables|Default|GetcurBulletCount) 2)
            (Variables|/Script/AdvancedWidgets.RadialSlider|SetValue _radialslider_93 0.66)))
        (:then_2
          (if (== (Variables|Default|GetcurBulletCount) 1)
            (Variables|/Script/AdvancedWidgets.RadialSlider|SetValue _radialslider_93 0.33)))
        (:then_3
          (if (== (Variables|Default|GetcurBulletCount) 0)
            (Variables|/Script/AdvancedWidgets.RadialSlider|SetValue _radialslider_93 0.0)))))))

(event EventResetKnifeLocation
  (bind _cutterknifecomp (Variables|Default|GetCutterKnifeComp))
  (Utilities|FlowControl|Delay 0.3)
  (Components|MoveComponentTo _cutterknifecomp (Variables|/Script/Engine.SceneComponent|GetRelativeLocation _cutterknifecomp) "-51.730000,69.428000,-67.260000" false false 0.15 false))

(event EventSetImageAlphaforHP
  (bind _curhp (Variables|Default|GetcurHP))
  (bind _hpuirefr (Variables|Default|GetHPUIRefR))
  (bind _radialslider_93 (Variables|/Game/KHJContents/UI/WB_HPUIR.WB_HPUIR_C|GetRadialSlider_93 _hpuirefr))
  (Utilities|FlowControl|Sequence
    (:then_0
      (if (== _curhp 3)
        (Variables|/Script/AdvancedWidgets.RadialSlider|SetValue _radialslider_93 1.0)))
    (:then_1
      (if (== _curhp 2)
        (Variables|/Script/AdvancedWidgets.RadialSlider|SetValue _radialslider_93 0.66)))
    (:then_2
      (if (== _curhp 1)
        (Variables|/Script/AdvancedWidgets.RadialSlider|SetValue _radialslider_93 0.33)))
    (:then_3
      (if (== _curhp 0)
        (Variables|/Script/AdvancedWidgets.RadialSlider|SetValue _radialslider_93 0.0)))))

(event EventResetKnifeCoolDown
  (Utilities|FlowControl|Delay 0.6)
  (Variables|Default|SetbCanFire true))

(event EventSetImageAlphaforCurBullets
  (bind _bulcountref (Variables|Default|GetBulCountRef))
  (bind _curbulletcount (Variables|Default|GetcurBulletCount))
  (bind _radialslider_93 (Variables|/Game/KHJContents/UI/WB_BulCountUIR.WB_BulCountUIR_C|GetRadialSlider_93 _bulcountref))
  (Variables|/Script/UMG.TextBlock|SetText (Variables|/Game/KHJContents/UI/WB_BulCountNum.WB_BulCountNum_C|Getcurbultext (Variables|Default|GetBulCountNumRef)) (Utilities|Text|ToText(Integer) _curbulletcount))
  (Utilities|FlowControl|Sequence
    (:then_0
      (if (== _curbulletcount 3)
        (Variables|/Script/AdvancedWidgets.RadialSlider|SetValue _radialslider_93 1.0)))
    (:then_1
      (if (== _curbulletcount 2)
        (Variables|/Script/AdvancedWidgets.RadialSlider|SetValue _radialslider_93 0.66)))
    (:then_2
      (if (== _curbulletcount 1)
        (Variables|/Script/AdvancedWidgets.RadialSlider|SetValue _radialslider_93 0.33)))
    (:then_3
      (if (== _curbulletcount 0)
        (Variables|/Script/AdvancedWidgets.RadialSlider|SetValue _radialslider_93 0.0)))))

(fn ConstructionScript)